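; Patrol bot Blueprint that walks an AI-driven loop along the points of a referenced spline path.
; MoveToNext sends AI MoveTo to the current point's local-space location, then on success waits briefly, advances the index and calls itself.
; The index wraps after a hard-coded four points, and failed moves are not handled.
; Nothing connected in this file starts the loop, as BeginPlay only calls its parent.
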(event `self.ReceiveBeginPlay`
  (`parent.ReceiveBeginPlay`))

(event `MoveToNext`
  ; AI Movement
  (`|AIMoveTo` null (`SplineComponent.GetLocationAtSplinePoint` (`/Game/01_Common/BP_BotPath.Spline` (`self.PathReference`)) (`self.CurrentPointIndex`) "Local") null
    (:`OnSuccess`
      (`KismetSystemLibrary.Delay` 1.0)
      (bind _result (`/Engine/EditorBlueprintResources/StandardMacros.IncrementInt` (`self.CurrentPointIndex`))
        (:`  `
          (if (> _result 3)
            (set `self.CurrentPointIndex` 0))
          (`self.MoveToNext`))))))

(fn `UserConstructionScript`
  (`parent.UserConstructionScript`))