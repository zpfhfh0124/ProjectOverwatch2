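; Overwatch-style Genji player character with shuriken attacks, a katana and first/third-person bone hiding.
; Shurikens spawn dormant on hand-mesh sockets, then left click fires them on a looping timer and right click fans them by socket.
; Both attacks share BurstTick, which updates PlayerState ammo; sets respawn while ammo remains, and R reloads.
; The katana spawns attached but hidden without collision, and E only plays its reflection montage.
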(event `self.ReceiveBeginPlay`
  (bind _asoverwatch_player_state (cast `OverwatchPlayerState` (`GameplayStatics.GetPlayerState` 0)))
  (set `self.OverwatchPlayerState` _asoverwatch_player_state)
  (`self.HideSkeletalMesh` true)
  (`self.ReLoadShuriken`)
  (`self.SpawnKatana`))

(event `self.ReceiveTick`
  (params (DeltaSeconds :type "Float (single-precision)")))

(event `self.OnMouseLB`
  (`self.AttackBurstFire`))

(event `self.OnMouseRB`
  (`self.AttackFanFire`)
  (`KismetSystemLibrary.Delay` 1.0)
  (set `self.IsFiring` false)
  (`self.ReSpawnShuriken`))

(event `self.OnR`
  (`self.ReLoadShuriken`))

(event `self.TogglePerspective`
  (`parent.TogglePerspective`)
  (switch `EPerspectiveMode` (`self.GetPerspectiveMode`)
    (:`FirstPerson`
      (`self.HideSkeletalMesh` true))
    (:`ThirdPerson`
      (`self.HideSkeletalMesh` false))))

(event `self.OnE`
  (`self.AttackReflection`))

(fn `AttackBlade`)

(fn `AttackBurstFire`
  (locals (BurstInterval :type "Float (double-precision)" :default 0.2))
  (if (`self.IsFiring`)
    (`KismetSystemLibrary.LogString` "이미 수리검 공격중인 상태이다")
    (else
      (set `self.IsFiring` true)
      (set `self.BurstIndex` 0)
      (`self.PlayAnimMontage` "/Game/GT/Genji/NewGenji/Anims/Genji_Shuriken_Cut_Montage.Genji_Shuriken_Cut_Montage")
      (set `self.ShootDir` (`self.GetForwardDir`))
      (bind _returnvalue (`KismetSystemLibrary.K2_SetTimerDelegate` (`|CreateDelegate` :!event `BurstTick`) (`local.BurstInterval`) true))
      (set `self.BurstTimerHandle` _returnvalue))))

(fn `AttackFanFire`
  (locals (Angle :type "Float (double-precision)") (AimDir :type "Vector Structure"))
  (bind (_aimdir_x _aimdir_y _aimdir_z) (`KismetMathLibrary.BreakVector` (`local.AimDir`)))
  (if (`self.IsFiring`)
    (`KismetSystemLibrary.LogString` "이미 수리검 공격중인 상태이다")
    (else
      (set `self.IsFiring` true)
      (set `self.BurstIndex` 0)
      (`self.PlayAnimMontage` "/Game/GT/Genji/NewGenji/Anims/Genji_Shuriken_Cut_Montage.Genji_Shuriken_Cut_Montage")
      (for _array_element (`self.ShurikenList`)
        (set `local.AimDir` (`self.GetForwardDir`))
        (switch `name` (`Shuriken.AttachedSocketName` _array_element)
          (:`Default`
            (`KismetSystemLibrary.PrintString` (`KismetStringLibrary.Concat_StrStr` "알 수 없는 소켓 Name이 들어가있다." (`KismetStringLibrary.Conv_NameToString` (`Shuriken.AttachedSocketName` _array_element)))))
          (:`ShurikenSocket_0`
            (set `local.Angle` 100.0)
            (set `self.ShootDir` (`KismetMathLibrary.MakeVector` _aimdir_x (+ _aimdir_y (`local.Angle`)) _aimdir_z) :!label _label)
            (`self.BurstTick`))
          (:`ShurikenSocket_1`
            (set `local.Angle` 0.0)
            (goto _label))
          (:`ShurikenSocket_2`
            (set `local.Angle` -100.0)
            (goto _label))))
      (`KismetArrayLibrary.Array_Clear` (`self.ShurikenList`)))))

(fn `AttackReflection`
  (`self.Katana`
    (:`then`
      (`self.PlayAnimMontage` "/Game/GT/Genji/Animations/Genji_Katana_Anim_Montage.Genji_Katana_Anim_Montage"))
    (:`else`
      (`KismetSystemLibrary.PrintString` "Katana is not valid"))))

(fn `BurstTick`
  (locals (Shuriken :type "/Game/GT/Genji/Shuriken/BP_Shuriken Object Reference"))
  (bind _shuriken (`local.Shuriken`))
  (if (>= (`self.BurstIndex`) (`KismetArrayLibrary.Array_Length` (`self.ShurikenList`)))
    (`KismetSystemLibrary.K2_ClearAndInvalidateTimerHandle` (`self.BurstTimerHandle`))
    (set `self.IsFiring` false)
    (`KismetArrayLibrary.Array_Clear` (`self.ShurikenList`))
    (`self.ReSpawnShuriken`)
    (else
      (bind _output_get (set `local.Shuriken` (`|GetArrayItem` (`self.ShurikenList`) (`self.BurstIndex`))))
      (`/Engine/EditorBlueprintResources/StandardMacros.IsValid` _output_get
        (:`Is Valid`
          (`self.SetActorScale3D` _shuriken (* (`self.GetActorScale3D` _shuriken) 4))
          (`Shuriken.FireInDirection` (`local.Shuriken`) (`self.ShootDir`))
          (bind _result (`/Engine/EditorBlueprintResources/StandardMacros.IncrementInt` (`self.BurstIndex`))
            (:`  `
              (set `self.BurstIndex` _result)
              (bind _result_2 (`/Engine/EditorBlueprintResources/StandardMacros.DecrementInt` (`self.ShurikenCount`))
                (:`  `
                  (bind _output_get_2 (set `self.ShurikenCount` _result_2))
                  (`OverwatchPlayerState.SetProjectileCurrCount` (`self.OverwatchPlayerState`) _output_get_2)
                  (`KismetSystemLibrary.PrintString` (`KismetStringLibrary.Concat_StrStr` "잔여 수리검 : " (`KismetStringLibrary.Conv_IntToString` _output_get_2))))))))
        (:`Is Not Valid`
          (bind _result_3 (`/Engine/EditorBlueprintResources/StandardMacros.IncrementInt` (`self.BurstIndex`))
            (:`  `
              (set `self.BurstIndex` _result_3))))))))

(fn `EquipKatana`
  (params (Equip :type Boolean))
  (bind _returnvalue (not Equip))
  (bind _boxcomp (`Katana.BoxComp` (`self.Katana`)))
  (`self.SetActorHiddenInGame` (`self.Katana`) _returnvalue)
  (if _returnvalue
    (`PrimitiveComponent.SetCollisionEnabled` _boxcomp "NoCollision")
    (else
      (`PrimitiveComponent.SetCollisionEnabled` _boxcomp "QueryAndPhysics"))))

(fn `HideSkeletalMesh`
  (params (Hide :type Boolean))
  (if Hide
    (for _array_element (`self.HideBoneNames`)
      (`SkinnedMeshComponent.HideBoneByName` (`self.Mesh`) _array_element "PBO_None"))
    (else
      (for _array_element_2 (`self.HideBoneNames`)
        (`SkinnedMeshComponent.UnHideBoneByName` (`self.Mesh`) _array_element_2)))))

(fn `ReLoadShuriken`
  (bind _output_get (set `self.ShurikenCount` (`self.ShurikenMax`)))
  (`OverwatchPlayerState.SetProjectileMaxCount` (`self.OverwatchPlayerState`) _output_get)
  (`self.SpawnShurikens`))

(fn `ReSpawnShuriken`
  (if (and (< (`self.ShurikenCount`) (`self.ShurikenMax`)) (> (`self.ShurikenCount`) 0))
    (`self.SpawnShurikens`)
    (else
      (`KismetSystemLibrary.PrintString` "ShurikenCount가 0이다.  추가 리로드 실행 필요"))))

(fn `SetAimWidget`
  (bind _returnvalue (`|CreateWidget` "/Game/FirstPerson/Blueprints/WBP_Crosshair.WBP_Crosshair_C" (`GameplayStatics.GetPlayerController` 0)))
  (`UserWidget.AddToViewport` _returnvalue 0))

(fn `SpawnKatana`
  (bind _returnvalue (`|SpawnActorFromClass` "/Game/GT/Genji/Katana/BP_Katana.BP_Katana_C" (`SceneComponent.GetSocketTransform` (`self.Mesh`) (`self.KatanaSocketName`) "RTS_ParentBoneSpace") "AdjustIfPossibleButAlwaysSpawn" "MultiplyWithRoot" null null))
  (bind _output_get (set `self.Katana` _returnvalue))
  (`self.K2_AttachToComponent` _output_get (`self.Mesh`) (`self.KatanaSocketName`) "SnapToTarget" "SnapToTarget" "KeepWorld" true)
  (`PrimitiveComponent.IgnoreActorWhenMoving` (`self.CapsuleComponent`) (`self.Katana`) false)
  (`self.EquipKatana` false))

(fn `SpawnShurikens`
  (locals (NewLocalVar :type "Array of Name") (NewLocalVar_0 :type "Array of Name") (Shuriken :type "/Game/GT/Genji/Shuriken/BP_Shuriken Object Reference"))
  (`KismetArrayLibrary.Array_Clear` (`self.ShurikenList`))
  (for (_array_element _array_index) (`self.ShurikenSocketNames`)
    (bind _returnvalue (`|SpawnActorFromClass` "/Game/GT/Genji/Shuriken/BP_Shuriken.BP_Shuriken_C" (`SceneComponent.GetSocketTransform` (`self.Mesh`) _array_element "RTS_World") "AdjustIfPossibleButAlwaysSpawn" "MultiplyWithRoot" null null))
    (bind _output_get (set `local.Shuriken` _returnvalue))
    (`self.SetOwner` _returnvalue (`GameplayStatics.GetPlayerCharacter` 0))
    (`ActorComponent.SetActive` (`Shuriken.ProjectileMovement` _output_get) false false)
    (`Shuriken.SetSocketName` (`local.Shuriken`) _array_element)
    (bind _returnvalue_2 (`self.K2_AttachToComponent` (`local.Shuriken`) (`self.Mesh`) _array_element "SnapToTarget" "SnapToTarget" "SnapToTarget" true))
    (if _returnvalue_2
      (`KismetArrayLibrary.Array_Insert` (`self.ShurikenList`) (`local.Shuriken`) _array_index)
      (`self.SetActorScale3D` (`local.Shuriken`) (/ (`self.GetActorScale3D` (`local.Shuriken`)) 4))
      (else
        (`KismetSystemLibrary.LogString` (`KismetStringLibrary.Concat_StrStr` (`KismetSystemLibrary.MakeLiteralString` (`KismetStringLibrary.Conv_NameToString` _array_element)) "에  Attach 되지 않았다"))))))

(fn `UserConstructionScript`)